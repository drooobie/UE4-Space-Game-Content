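; BP_Tree is a generic tree node with parent and child links, addressed by integer index paths.
; Set, AddChild and Remove find the parent through GetParent and recursive Get, while MakeRectangular recursively sizes children from per-depth dimensions.
; Iterate recursively calls an iterator body, with options for order and leaves only.
; It looks unfinished: Get always reads the first index, loop bounds stay at zero and ToString returns empty.
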(event Custom|CustomEvent_0)

(fn Get
  (params (Index :type Array%20of%20Integers) (Depth :type Integer))
  (if (== (Utilities|Array|Length Index) 0)
    (return self)
    (else
      (bind _node (CallFunction|Get (Utilities|Array|Get(acopy) (Variables|Default|GetChildren) (Utilities|Array|Get(acopy) Index)) Index (+ Depth 1)))
      (return _node))))

(fn Set
  (params (Node :type BP%20Tree%20Object%20Reference) (Index :type Array%20of%20Integers))
  (bind _parentnode (CallFunction|GetParent Index))
  (Variables|BP_Tree_C|SetParent Node _parentnode)
  (Utilities|Array|SetArrayElem (Variables|BP_Tree_C|GetChildren _parentnode) (Utilities|Array|Get(acopy) Index (Utilities|Array|LastIndex Index)) Node))

(fn AddChild
  (params (Node :type BP%20Tree%20Object%20Reference) (Index :type Array%20of%20Integers))
  (bind _parentnode (CallFunction|GetParent Index))
  (Variables|BP_Tree_C|SetParent Node _parentnode)
  (Utilities|Array|Add (Variables|BP_Tree_C|GetChildren _parentnode) Node))

(fn Remove
  (params (Index :type Array%20of%20Integers))
  (bind _parentnode (CallFunction|GetParent Index))
  (bind _output_get (LocalVariables|SetReturnValue (Utilities|Array|Get(acopy) (Variables|BP_Tree_C|GetChildren _parentnode))))
  (Utilities|Array|RemoveIndex (Variables|BP_Tree_C|GetChildren _parentnode) (Utilities|Array|Get(acopy) Index (Utilities|Array|LastIndex Index)))
  (return _output_get))

(fn GetParent
  (params (Index :type Array%20of%20Integers))
  (bind _returnvalue (Utilities|Array|LastIndex Index))
  (LocalVariables|SetLastIndex (Utilities|Array|Get(acopy) Index _returnvalue))
  (Utilities|Array|RemoveIndex Index _returnvalue)
  (bind _node (CallFunction|Get Index))
  (return _node))

(fn Iterate
  (params (LoopBody :type BP%20Function%20Tree%20Object%20Reference) (NumChildrenBeforeParent :type Integer) (Reverse :type Boolean) (LeavesOnly :type Boolean) (Index :type Array%20of%20Integers))
  (LocalVariables|SetNumChildren (Utilities|Array|Length (Variables|Default|GetChildren)))
  ;[1 1 1] Set Up Loop Indices for Left
  (if Reverse
    (LocalVariables|SetFirstIndex (- (LocalVariables|GetNumChildren) 1))
    (LocalVariables|SetLastIndex (Math|Integer|Max(Integer) (- (LocalVariables|GetNumChildren) NumChildrenBeforeParent)))
    (LocalVariables|SetStep -1)
    (else
      (LocalVariables|SetFirstIndex 0)
      (LocalVariables|SetLastIndex (- (Math|Integer|Max(Integer) NumChildrenBeforeParent (LocalVariables|GetNumChildren)) 1))
      (LocalVariables|SetStep 1)))
  ;[1 1 1] Execute "Left" Children
  (bind _value (Utilities|RangeLoop 0 0 (LocalVariables|GetStep))
    (:LoopBody
      (Utilities|Array|Add Index _value)
      (CallFunction|Iterate (Utilities|Array|Get(acopy) (Variables|Default|GetChildren) _value) LoopBody NumChildrenBeforeParent Reverse LeavesOnly Index))
    (:Completed
      ;[1 1 1] Execute Current Node
      (if LeavesOnly
        (if (== (LocalVariables|GetNumChildren) 0)
          (Default|CallIteratorBody self Index :!label _label)
          ;[1 1 1] Set Up Loop Indices for Right
          (LocalVariables|SetFirstIndex (+ (LocalVariables|GetLastIndex) (LocalVariables|GetStep)))
          (if true
            (LocalVariables|SetLastIndex 0)
            (else
              (LocalVariables|SetLastIndex (- (LocalVariables|GetNumChildren) 1))))
          ;[1 1 1] Execute "Right" Children
          (bind _value_2 (Utilities|RangeLoop 0 0 (LocalVariables|GetStep))
            (:LoopBody
              (Utilities|Array|Add Index _value_2)
              (CallFunction|Iterate (Utilities|Array|Get(acopy) (Variables|Default|GetChildren) _value_2) LoopBody NumChildrenBeforeParent Reverse LeavesOnly Index))
            (:Completed
              (if (> (Utilities|Array|Length Index) 0)
                (Utilities|Array|RemoveIndex Index (Utilities|Array|LastIndex Index))))))
        (else
          (goto _label))))))

(fn MakeRectangular
  (params (Dimensions :type Array%20of%20Integers) (Depth :type Integer))
  (bind _children (Variables|Default|GetChildren))
  (Utilities|Array|Clear _children)
  (Utilities|Array|Resize _children (Utilities|Array|Get(acopy) Dimensions Depth))
  (for _array_element _children
    (CallFunction|MakeRectangular _array_element Dimensions (+ Depth 1))))

(fn ToString
  (return ""))