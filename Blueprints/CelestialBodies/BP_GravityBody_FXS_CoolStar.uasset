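; A cool star celestial body with configurable surface, atmosphere, corona and flare visuals, plus a gravity Forcer component.
; The construction script scales the actor and fluid settings from FinalRadius, then drives dynamic materials on the star mesh, corona plates and particle flares.
; BeginPlay passes radius and mass to the Forcer, overrides the mesh's physics mass to zero and applies InitialVelocity.
; When IsMovable is false, Tick pins location, rotation and velocity.
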(event EventBeginPlay
  (bind _star (Variables|Default|GetStar))
  (Variables|/Game/Self/Blueprints/Components/Forcers/BPC_ForcerRadial.BPC_ForcerRadial_C|SetInnerRadius (Variables|Default|GetForcer) (Variables|Default|GetFinalRadius))
  (Variables|/Game/Self/Blueprints/Components/Forcers/BPC_ForcerGravity_ITW.BPC_ForcerGravity_ITW_C|SetMass (Variables|Default|GetForcer) (Variables|Default|GetMass))
  (Class|PrimitiveComponent|SetMassOverrideinKg _star "None" 0.0 true)
  (Physics|SetPhysicsLinearVelocity _star (Variables|Default|GetInitialVelocity) false "None")
  (Variables|Default|SetInitialPosition (Transformation|GetActorLocation)))

(event Collision|EventActorBeginOverlap
  (params (OtherActor :type Actor%20Object%20Reference)))

(event EventTick
  (params (DeltaSeconds :type Float%20%28single-precision%29))
  (if (not (Variables|Default|GetIsMovable))
    (Transformation|SetActorRotation "0, 0, 0")
    (Transformation|SetActorLocation (Variables|Default|GetInitialPosition) false false)
    (Physics|SetPhysicsLinearVelocity (Variables|Default|GetStar) "0, 0, 0" false "None")))

(fn ConstructionScript
  (Utilities|FlowControl|Sequence
    (:then_0
      (LocalVariables|SetScaleAmount (/ (Variables|Default|GetFinalRadius) 2.6e+03))
      (Variables|ScaledStarProperties|SetScaledFluidResolution (* (Variables|StarProperties|GetFluid_Resolution) (LocalVariables|GetScaleAmount)))
      (Transformation|SetActorScale3D self (Math|Conversions|ToVector(Float) (LocalVariables|GetScaleAmount)))
      (Variables|ScaledStarProperties|SetScaledFluidDensity (* (Variables|StarProperties|GetFluid_Density) (LocalVariables|GetScaleAmount))))
    (:then_1
      (Utilities|Array|Clear (Variables|Default|GetStarFlares))
      (Utilities|Array|Clear (Variables|Default|GetStarPlates)))
    (:then_2
      (bind _returnvalue (Rendering|Material|CreateDynamicMaterialInstance (Variables|Default|GetStar) 0 0 :!class /Script/Engine.PrimitiveComponent))
      (Variables|Default|SetStar_DM_A _returnvalue)
      (Utilities|FlowControl|Sequence
        (:then_0
          (Rendering|Material|SetVectorParameterValue (Variables|Default|GetStar_DM_A) "KL_AtmoCool" (Variables|StarProperties|GetAtmosphere_Kelvin) :!class /Script/Engine.MaterialInstanceDynamic)
          (Rendering|Material|SetVectorParameterValue (Variables|Default|GetStar_DM_A) "KL_SurfaceCool" (Variables|StarProperties|GetSurfaceKelvin_Cool) :!class /Script/Engine.MaterialInstanceDynamic)
          (Rendering|Material|SetVectorParameterValue (Variables|Default|GetStar_DM_A) "KL_SurfaceWarm" (Variables|StarProperties|GetSurfaceKelvin_Warm) :!class /Script/Engine.MaterialInstanceDynamic)
          (Rendering|Material|SetVectorParameterValue (Variables|Default|GetStar_DM_A) "KL_SurfaceHot" (Variables|StarProperties|GetSurfaceKelvin_Hot) :!class /Script/Engine.MaterialInstanceDynamic)
          (Rendering|Material|SetVectorParameterValue (Variables|Default|GetStar_DM_A) "SurfaceActivity_Bleed" (Variables|StarProperties|GetSurface_Bleed) :!class /Script/Engine.MaterialInstanceDynamic)
          (Rendering|Material|SetVectorParameterValue (Variables|Default|GetStar_DM_A) "SurfaceActivity_Center" (Variables|StarProperties|GetSurface_Spot) :!class /Script/Engine.MaterialInstanceDynamic))
        (:then_1
          (Rendering|Material|SetScalarParameterValue (Variables|Default|GetStar_DM_A) "3DCoord_FlowTile" (Variables|ScaledStarProperties|GetScaledFluidResolution) :!class /Script/Engine.MaterialInstanceDynamic)
          (Rendering|Material|SetScalarParameterValue (Variables|Default|GetStar_DM_A) "3DFlowNormal_Power" (Variables|ScaledStarProperties|GetScaledFluidDensity) :!class /Script/Engine.MaterialInstanceDynamic)
          (Rendering|Material|SetScalarParameterValue (Variables|Default|GetStar_DM_A) "3DPlasmaFlow_Speed" (Variables|StarProperties|GetFluid_Speed) :!class /Script/Engine.MaterialInstanceDynamic)
          (Rendering|Material|SetScalarParameterValue (Variables|Default|GetStar_DM_A) "3DSurface_Offset" (Variables|StarProperties|GetSurface_Offset) :!class /Script/Engine.MaterialInstanceDynamic)
          (Rendering|Material|SetScalarParameterValue (Variables|Default|GetStar_DM_A) "DistAtmo_Falloff" (Variables|StarProperties|GetAtmosphere_Curve) :!class /Script/Engine.MaterialInstanceDynamic)
          (Rendering|Material|SetScalarParameterValue (Variables|Default|GetStar_DM_A) "DistAtmo_Power" (Variables|StarProperties|GetAtmosphere_Density) :!class /Script/Engine.MaterialInstanceDynamic))
        (:then_2
          (Rendering|Material|SetScalarParameterValue (Variables|Default|GetStar_DM_A) "FluidActivity_Influence" (Variables|StarProperties|GetStormSurface_Blend) :!class /Script/Engine.MaterialInstanceDynamic)
          (Rendering|Material|SetScalarParameterValue (Variables|Default|GetStar_DM_A) "SolarActivity_InnerFalloff" (Variables|StarProperties|GetStormIn_Curve) :!class /Script/Engine.MaterialInstanceDynamic)
          (Rendering|Material|SetScalarParameterValue (Variables|Default|GetStar_DM_A) "SolarActivity_OutsideFalloff" (Variables|StarProperties|GetStormOut_Curve) :!class /Script/Engine.MaterialInstanceDynamic)
          (Rendering|Material|SetScalarParameterValue (Variables|Default|GetStar_DM_A) "Tessellation_Resolution" (Variables|StarProperties|GetTessellation_Resolution) :!class /Script/Engine.MaterialInstanceDynamic)
          (Rendering|Material|SetScalarParameterValue (Variables|Default|GetStar_DM_A) "Vertex_Speed" (Variables|StarProperties|GetVertexSpeed_Animation) :!class /Script/Engine.MaterialInstanceDynamic)
          (Rendering|Material|SetScalarParameterValue (Variables|Default|GetStar_DM_A) "VertexOffset_Falloff" (Variables|StarProperties|GetVertex_Curve) :!class /Script/Engine.MaterialInstanceDynamic))
        (:then_3
          (Rendering|Material|SetScalarParameterValue (Variables|Default|GetStar_DM_A) "VertexOffset_Power" (Variables|StarProperties|GetVertex_Power) :!class /Script/Engine.MaterialInstanceDynamic)
          (Rendering|Material|SetScalarParameterValue (Variables|Default|GetStar_DM_A) "VertexOffset_Tile" (Variables|StarProperties|GetVertex_Resolution) :!class /Script/Engine.MaterialInstanceDynamic))))
    (:then_3
      (for _array_element (Actor|GetComponentsByClass "/Script/Engine.ParticleSystemComponent")
        (bind _returnvalue_2 (Rendering|Material|CreateDynamicMaterialInstance _array_element 0 0 :!class /Script/Engine.PrimitiveComponent))
        (Utilities|Array|Add (Variables|Default|GetStarFlares) _returnvalue_2)))
    (:then_4
      (for _array_element_2 (Actor|GetComponentsByClass "/Script/Engine.StaticMeshComponent")
        (if (!= _array_element_2 (Variables|Default|GetStar))
          (bind _returnvalue_3 (Rendering|Material|CreateDynamicMaterialInstance _array_element_2 0 0 :!class /Script/Engine.PrimitiveComponent))
          (Utilities|Array|Add (Variables|Default|GetStarPlates) _returnvalue_3))))
    (:then_5
      (for _array_element_3 (Variables|Default|GetStarPlates)
        (Rendering|Material|SetVectorParameterValue _array_element_3 "CoronaKelvin_Cool" (Variables|StarProperties|GetCorona_Kelvin) :!class /Script/Engine.MaterialInstanceDynamic)))
    (:then_6
      (for _array_element_4 (Variables|Default|GetStarFlares)
        (Rendering|Material|SetVectorParameterValue _array_element_4 "FlareColor" (Variables|StarProperties|GetFlare_KelvinOffset) :!class /Script/Engine.MaterialInstanceDynamic)))))