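; BP_FXS_HotStar is a hot star effect actor whose look is set up entirely in its construction script.
; A dynamic material on the StarHot mesh receives the surface, atmosphere, plasma flow, storm, tessellation and vertex animation settings.
; Other static meshes and all particle systems get dynamic materials cached in StarPlates and StarFlares.
; Final loops set corona and flare colors on material arrays; the event graph is unused.
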(event `self.ReceiveBeginPlay`)

(event `self.ReceiveActorBeginOverlap`
  (params (OtherActor :type "Actor Object Reference")))

(event `self.ReceiveTick`
  (params (DeltaSeconds :type "Float (single-precision)")))

(fn `UserConstructionScript`
  (bind _star_dm_b (`self.Star_DM_B`))
  (bind _star_dm_b_2 (`self.Star_DM_B`))
  (bind _star_dm_b_3 (`self.Star_DM_B`))
  (bind _star_dm_b_4 (`self.Star_DM_B`))
  (`|ExecutionSequence`
    (:`then_0`
      (`KismetArrayLibrary.Array_Clear` (`self.StarFlares`))
      (`KismetArrayLibrary.Array_Clear` (`self.StarPlates`)))
    (:`then_1`
      (bind _returnvalue (`PrimitiveComponent.CreateDynamicMaterialInstance` (`self.StarHot`) 0 null))
      (set `self.Star_DM_B` _returnvalue)
      (`|ExecutionSequence`
        (:`then_0`
          (`MaterialInstanceDynamic.SetVectorParameterValue` _star_dm_b "KH_AtmoHot" (`self.Atmosphere_Kelvin`))
          (`MaterialInstanceDynamic.SetVectorParameterValue` _star_dm_b "KH_SurfaceCool" (`self.SurfaceKelvin_Cool`))
          (`MaterialInstanceDynamic.SetVectorParameterValue` _star_dm_b "KH_SurfaceWarm" (`self.SurfaceKelvin_Warm`))
          (`MaterialInstanceDynamic.SetVectorParameterValue` _star_dm_b "KH_SurfaceHot" (`self.SurfaceKelvin_Hot`))
          (`MaterialInstanceDynamic.SetVectorParameterValue` _star_dm_b "SurfaceActivity_Bleed" (`self.Surface_Bleed`))
          (`MaterialInstanceDynamic.SetVectorParameterValue` _star_dm_b "SurfaceActivity_Center" (`self.Surface_Spot`)))
        (:`then_1`
          (`MaterialInstanceDynamic.SetScalarParameterValue` _star_dm_b_2 "3DCoord_FlowTile" (`self.Fluid_Resolution`))
          (`MaterialInstanceDynamic.SetScalarParameterValue` _star_dm_b_2 "3DFlowNormal_Power" (`self.Fluid_Density`))
          (`MaterialInstanceDynamic.SetScalarParameterValue` _star_dm_b_2 "3DPlasmaFlow_Speed" (`self.Fluid_Speed`))
          (`MaterialInstanceDynamic.SetScalarParameterValue` _star_dm_b_2 "3DSurface_Offset" (`self.Surface_Offset`))
          (`MaterialInstanceDynamic.SetScalarParameterValue` _star_dm_b_2 "DistAtmo_Falloff" (`self.Atmosphere_Curve`))
          (`MaterialInstanceDynamic.SetScalarParameterValue` _star_dm_b_2 "DistAtmo_Power" (`self.Atmosphere_Density`)))
        (:`then_2`
          (`MaterialInstanceDynamic.SetScalarParameterValue` _star_dm_b_3 "FluidActivity_Influence" (`self.StormSurface_Blend`))
          (`MaterialInstanceDynamic.SetScalarParameterValue` _star_dm_b_3 "SolarActivity_InnerFalloff" (`self.StormIn_Curve`))
          (`MaterialInstanceDynamic.SetScalarParameterValue` _star_dm_b_3 "SolarActivity_OutsideFalloff" (`self.StormOut_Curve`))
          (`MaterialInstanceDynamic.SetScalarParameterValue` _star_dm_b_3 "Tessellation_Resolution" (`self.Tessellation_Resolution`))
          (`MaterialInstanceDynamic.SetScalarParameterValue` _star_dm_b_3 "Vertex_Speed" (`self.VertexSpeed_Animation`))
          (`MaterialInstanceDynamic.SetScalarParameterValue` _star_dm_b_3 "VertexOffset_Falloff" (`self.Vertex_Curve`)))
        (:`then_3`
          (`MaterialInstanceDynamic.SetScalarParameterValue` _star_dm_b_4 "VertexOffset_Power" (`self.Vertex_Power`))
          (`MaterialInstanceDynamic.SetScalarParameterValue` _star_dm_b_4 "VertexOffset_Tile" (`self.Vertex_Resolution`)))))
    (:`then_2`
      (for _array_element (`self.K2_GetComponentsByClass` "/Script/Engine.ParticleSystemComponent")
        (bind _returnvalue_2 (`PrimitiveComponent.CreateDynamicMaterialInstance` _array_element 0 null))
        (`KismetArrayLibrary.Array_Add` (`self.StarFlares`) _returnvalue_2)))
    (:`then_3`
      (for _array_element_2 (`self.K2_GetComponentsByClass` "/Script/Engine.StaticMeshComponent")
        (if (!= _array_element_2 (`self.StarHot`))
          (bind _returnvalue_3 (`PrimitiveComponent.CreateDynamicMaterialInstance` _array_element_2 0 null))
          (`KismetArrayLibrary.Array_Add` (`self.StarPlates`) _returnvalue_3))))
    (:`then_4`
      (for _array_element_3 _
        (`MaterialInstanceDynamic.SetVectorParameterValue` _array_element_3 "CoronaKelvin_Hot" (`self.Corona_Kelvin`))))
    (:`then_5`
      (for _array_element_4 _
        (`MaterialInstanceDynamic.SetVectorParameterValue` _array_element_4 "FlareColor" (`self.Flare_KelvinOffset`))))))