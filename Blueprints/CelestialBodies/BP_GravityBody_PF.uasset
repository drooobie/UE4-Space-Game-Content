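; BP_GravityBody_PF is a celestial body actor that carries mass, radius and an initial velocity for physics-based gravity.
; The construction script scales the actor by the ratio of final to initial radius.
; On BeginPlay it passes radius and mass to its Forcer component, overrides the mesh mass and applies the starting velocity.
; Bodies flagged as not movable are pinned each tick by resetting position and zeroing linear velocity.
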(event `self.ReceiveBeginPlay`
  (bind _forcer (`self.Forcer`))
  (bind _staticmesh (`self.StaticMesh`))
  (set `/Game/Self/Blueprints/Components/Forcers/BPC_ForcerRadial.InnerRadius` (`self.FinalRadius`) _forcer)
  (bind _output_get (set `/Game/Self/Blueprints/Components/Forcers/BPC_ForcerGravity_ITW.Mass` (`self.Mass`) _forcer))
  (`PrimitiveComponent.SetMassOverrideInKg` _staticmesh "None" _output_get true)
  (`PrimitiveComponent.SetPhysicsLinearVelocity` _staticmesh (`self.InitialVelocity`) false "None")
  (set `self.InitialPosition` (`self.K2_GetActorLocation`)))

(event `self.ReceiveTick`
  (params (DeltaSeconds :type "Float (single-precision)"))
  (if (not (`self.IsMovable`))
    (`self.K2_SetActorLocation` (`self.InitialPosition`))
    (`PrimitiveComponent.SetPhysicsLinearVelocity` (`self.StaticMesh`) (0.0 0.0 0.0) false "None")))

(event `self.ReceiveActorBeginOverlap`
  (params (OtherActor :type "Actor Object Reference")))

(fn `StampRadius`)

(fn `UserConstructionScript`
  (`self.SetActorScale3D` (`KismetMathLibrary.Conv_DoubleToVector` (/ (`self.FinalRadius`) (`self.InitialRadius`)))))