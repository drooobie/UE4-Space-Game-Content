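; Procedural planet actor that colors its sphere mesh's atmosphere, oceans, terrain and polar regions from color variables.
; All work happens in the Construction Script, where UseStaticParameters selects the material path.
; When true, it applies M_PlanetMasterMPC and writes the colors to the shared MPC_Planet collection, so planets on this path share one palette.
; Otherwise, it sets them on a per-actor dynamic instance of M_PlanetMaster_Inst.
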(event `self.ReceiveBeginPlay`)

(event `self.ReceiveActorBeginOverlap`
  (params (OtherActor :type "Actor Object Reference")))

(event `self.ReceiveTick`
  (params (DeltaSeconds :type "Float (single-precision)")))

(fn `UserConstructionScript`
  (bind _atmospherecolor (`self.AtmosphereColor`))
  (bind _deepoceancolor (`self.DeepOceanColor`))
  (bind _grasscolor (`self.GrassColor`))
  (bind _groundcolor (`self.GroundColor`))
  (bind _mountaincolor (`self.MountainColor`))
  (bind _oceancolor (`self.OceanColor`))
  (bind _polarcolor (`self.PolarColor`))
  (if (`self.UseStaticParameters`)
    (`PrimitiveComponent.CreateDynamicMaterialInstance` (`self.SphereMesh`) 0 "/Game/Self/Materials/CelestialBodies/M_PlanetMasterMPC.M_PlanetMasterMPC")
    (`KismetMaterialLibrary.SetVectorParameterValue` "/Game/Self/Materials/ParameterCollections/MPC_Planet.MPC_Planet" "AtmosphereColor" _atmospherecolor)
    (`KismetMaterialLibrary.SetVectorParameterValue` "/Game/Self/Materials/ParameterCollections/MPC_Planet.MPC_Planet" "DeepOceanColor" _deepoceancolor)
    (`KismetMaterialLibrary.SetVectorParameterValue` "/Game/Self/Materials/ParameterCollections/MPC_Planet.MPC_Planet" "GrassColor" _grasscolor)
    (`KismetMaterialLibrary.SetVectorParameterValue` "/Game/Self/Materials/ParameterCollections/MPC_Planet.MPC_Planet" "GroundColor" _groundcolor)
    (`KismetMaterialLibrary.SetVectorParameterValue` "/Game/Self/Materials/ParameterCollections/MPC_Planet.MPC_Planet" "MountainColor" _mountaincolor)
    (`KismetMaterialLibrary.SetVectorParameterValue` "/Game/Self/Materials/ParameterCollections/MPC_Planet.MPC_Planet" "OceanColor" _oceancolor)
    (`KismetMaterialLibrary.SetVectorParameterValue` "/Game/Self/Materials/ParameterCollections/MPC_Planet.MPC_Planet" "PolarColor" _polarcolor)
    (else
      (bind _returnvalue (`PrimitiveComponent.CreateDynamicMaterialInstance` (`self.SphereMesh`) 0 "/Game/Self/Materials/CelestialBodies/M_PlanetMaster_Inst.M_PlanetMaster_Inst"))
      (`MaterialInstanceDynamic.SetVectorParameterValue` _returnvalue "AtmosphereColor" _atmospherecolor)
      (`MaterialInstanceDynamic.SetVectorParameterValue` _returnvalue "DeepOceanColor" _deepoceancolor)
      (`MaterialInstanceDynamic.SetVectorParameterValue` _returnvalue "GrassColor" _grasscolor)
      (`MaterialInstanceDynamic.SetVectorParameterValue` _returnvalue "GroundColor" _groundcolor)
      (`MaterialInstanceDynamic.SetVectorParameterValue` _returnvalue "MountainColor" _mountaincolor)
      (`MaterialInstanceDynamic.SetVectorParameterValue` _returnvalue "OceanColor" _oceancolor)
      (`MaterialInstanceDynamic.SetVectorParameterValue` _returnvalue "PolarColor" _polarcolor))))