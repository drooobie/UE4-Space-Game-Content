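; Actor that feeds gravity well positions to the grid material, presumably so the grid can respond to them.
; Every tick it reads GravityWellActors from BP_GameState_ITW and writes each location into its numbered vector parameter in the MPC_GridWells collection, supporting up to eight wells.
; The construction script creates a dynamic instance of the emissive grid material on its Sphere.
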(event `self.ReceiveBeginPlay`)

(event `self.ReceiveActorBeginOverlap`
  (params (OtherActor :type "Actor Object Reference")))

(event `self.ReceiveTick`
  (params (DeltaSeconds :type "Float (single-precision)"))
  (bind _asbp_game_state_itw (cast `/Game/Self/Blueprints/Gameplay/BP_GameState_ITW` (`GameplayStatics.GetGameState`)))
  (for (_array_element _array_index) (`/Game/Self/Blueprints/Gameplay/BP_GameState_ITW.GravityWellActors` _asbp_game_state_itw)
    (switch `int` _array_index
      (:`0`
        (bind _returnvalue (`KismetMathLibrary.Conv_VectorToLinearColor` (`self.K2_GetActorLocation` _array_element)))
        (`KismetMaterialLibrary.SetVectorParameterValue` "/Game/Self/Materials/ParameterCollections/MPC_GridWells.MPC_GridWells" "Gravity Well 1" _returnvalue))
      (:`1`
        (`KismetMaterialLibrary.SetVectorParameterValue` "/Game/Self/Materials/ParameterCollections/MPC_GridWells.MPC_GridWells" "Gravity Well 2" _returnvalue))
      (:`2`
        (`KismetMaterialLibrary.SetVectorParameterValue` "/Game/Self/Materials/ParameterCollections/MPC_GridWells.MPC_GridWells" "Gravity Well 3" _returnvalue))
      (:`3`
        (`KismetMaterialLibrary.SetVectorParameterValue` "/Game/Self/Materials/ParameterCollections/MPC_GridWells.MPC_GridWells" "Gravity Well 4" _returnvalue))
      (:`4`
        (`KismetMaterialLibrary.SetVectorParameterValue` "/Game/Self/Materials/ParameterCollections/MPC_GridWells.MPC_GridWells" "Gravity Well 5" _returnvalue))
      (:`5`
        (`KismetMaterialLibrary.SetVectorParameterValue` "/Game/Self/Materials/ParameterCollections/MPC_GridWells.MPC_GridWells" "Gravity Well 6" _returnvalue))
      (:`6`
        (`KismetMaterialLibrary.SetVectorParameterValue` "/Game/Self/Materials/ParameterCollections/MPC_GridWells.MPC_GridWells" "Gravity Well 7" _returnvalue))
      (:`7`
        (`KismetMaterialLibrary.SetVectorParameterValue` "/Game/Self/Materials/ParameterCollections/MPC_GridWells.MPC_GridWells" "Gravity Well 8" _returnvalue)))))

(fn `UserConstructionScript`
  (`PrimitiveComponent.CreateDynamicMaterialInstance` (`self.Sphere`) 0 "/Game/Self/Materials/Grid/MI_GridEmissiveCompute_MPC_01.MI_GridEmissiveCompute_MPC_01"))