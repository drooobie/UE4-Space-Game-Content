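; BP_PawnEffect is a base for pawn effects that fire repeatedly while activated.
; Start and Stop toggle activation, and each Tick call runs Effect when active and off cooldown.
; A positive EffectCooldown sets a cooldown flag before the effect runs and clears it by timer, while zero or less lets it fire every tick.
; Effect is empty here, leaving the behavior to overrides.
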(fn `Effect`)

(fn `ResetCooldown`
  (set `self.OnCooldown` false))

(fn `Start`
  (set `self.IsActivated` true))

(fn `Stop`
  (set `self.IsActivated` false))

(fn `Tick`
  (if (and (`self.IsActivated`) (not (`self.OnCooldown`)))
    (`|ExecutionSequence`
      (:`then_0`
        (if (> (`self.EffectCooldown`) 0.0)
          (set `self.OnCooldown` true)
          (`KismetSystemLibrary.K2_SetTimer` null "ResetCooldown" (`self.EffectCooldown`))))
      (:`then_1`
        (`self.Effect`)))))