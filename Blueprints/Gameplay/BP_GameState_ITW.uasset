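; BP_GameState_ITW is a game state Blueprint whose only live logic is a debug input hook.
; Pressing the DebugHandle action looks up the key in DebugKeys and passes its index plus one to the DebugHandler's ToggleDispatcher.
; BeginPlay, Tick and the construction script are empty.
; Disconnected scratch nodes remain for printing force receiver counts, testing rotation math and sampling random pairs from a range.
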(event `self.ReceiveBeginPlay`)

(event `self.ReceiveTick`
  (params (DeltaSeconds :type "Float (single-precision)")))

(event `InputAction|DebugHandle`
  (params (Key :type "Key Structure" :default "AnyKey"))
  (:`Pressed`
    (`/Game/Self/Blueprints/Engine/BP_DebugHandler.ToggleDispatcher` (`self.DebugHandler`) (+ (`KismetArrayLibrary.Array_Find` (`self.DebugKeys`) Key) 1))))

(fn `UserConstructionScript`)