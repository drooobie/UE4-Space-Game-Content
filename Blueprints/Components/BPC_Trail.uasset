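; Actor component that draws a debug-line trail along the path of its owning actor.
; It stores the owner's location at BeginPlay, then each Tick with Draw enabled draws a segment from that point to the current location and updates it.
; Color, thickness and lifetime come from variables.
; The stored point is frozen while Draw is off, so re-enabling it bridges the gap with one straight line.
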(event `self.ReceiveBeginPlay`
  (bind _output_get (set `self.Actor` (`self.GetOwner`)))
  (set `self.Location` (`Actor.K2_GetActorLocation` _output_get)))

(event `self.ReceiveTick`
  (params (DeltaSeconds :type "Float (single-precision)"))
  (bind _returnvalue (`Actor.K2_GetActorLocation` (`self.Actor`)))
  (if (`self.Draw`)
    (`KismetSystemLibrary.DrawDebugLine` (`self.Location`) _returnvalue (`self.Color`) (`self.Duration`) (`self.Thickness`))
    (set `self.Location` _returnvalue)))