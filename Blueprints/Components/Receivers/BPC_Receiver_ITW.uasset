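; Receiver component that registers itself with BP_GameState_ITW as a target for forces, which are applied by Forcers.
; If active when added to the game, it joins the Receivers list and binds to the game state's pre- and post-physics tick dispatchers; removal undoes both.
; The post-physics handler draws and resets the tick's force.
; The pre-physics handler and SetForcers are empty, and the receiver-side Forcers lookup is disconnected.
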(event `self.ReceiveBeginPlay`
  (`parent.ReceiveBeginPlay`))

(event `self.ReceiveTick`
  (params (DeltaSeconds :type "Float (single-precision)")))

(event `self.AddToGame`
  ;[1 1 1] If It Starts Off, It Stays Off
  (if (`self.IsActive`)
    (bind _asbp_game_state_itw (cast `/Game/Self/Blueprints/Gameplay/BP_GameState_ITW` (`GameplayStatics.GetGameState`)))
    (`KismetArrayLibrary.Array_Add` (`/Game/Self/Blueprints/Gameplay/BP_GameState_ITW.Receivers` _asbp_game_state_itw) self)
    (add `/Game/Self/Blueprints/Engine/BP_GameTickHandler.Dispatch2` (`/Game/Self/Blueprints/Gameplay/BP_GameState_ITW.TickPrePhysics` _asbp_game_state_itw) (delegate `TickH`))
    (add `/Game/Self/Blueprints/Engine/BP_GameTickHandler.Dispatch1` (`/Game/Self/Blueprints/Gameplay/BP_GameState_ITW.TickPostPhysics` _asbp_game_state_itw) (delegate `TickH2`))))

(event `TickH`
  (params (TickingGroup :type "ETickingGroup Enum") (Subgroup :type Integer)))

(event `TickH2`
  (params (TickingGroup :type "ETickingGroup Enum") (Subgroup :type Integer))
  (`self.DrawForce`)
  (`self.ResetTickForce`))

(event `self.RemoveFromGame`
  (bind _asbp_game_state_itw (cast `/Game/Self/Blueprints/Gameplay/BP_GameState_ITW` (`GameplayStatics.GetGameState`)))
  (`KismetArrayLibrary.Array_RemoveItem` (`/Game/Self/Blueprints/Gameplay/BP_GameState_ITW.Receivers` _asbp_game_state_itw) self)
  (remove `/Game/Self/Blueprints/Engine/BP_GameTickHandler.Dispatch2` (`/Game/Self/Blueprints/Gameplay/BP_GameState_ITW.TickPrePhysics` _asbp_game_state_itw) (delegate `TickH`))
  (remove `/Game/Self/Blueprints/Engine/BP_GameTickHandler.Dispatch1` (`/Game/Self/Blueprints/Gameplay/BP_GameState_ITW.TickPostPhysics` _asbp_game_state_itw) (delegate `TickH2`)))

(event `self.SetForcers`
  ;[1 1 1] Forces Applied In Forcers
)