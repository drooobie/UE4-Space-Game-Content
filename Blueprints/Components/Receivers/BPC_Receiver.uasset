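; Base receiver component that applies forces from a set of forcer objects to its owner's physics body.
; On BeginPlay it takes and wakes the owner's root primitive, then calls SetForcers and AddToGame, which are empty hooks here, as is RemoveFromGame on EndPlay.
; ReceiveFromAll queries each forcer's ForceFunction, applies the result and sums it into TickForce.
; DrawForce shows that total as a log-scaled debug line, and ResetTickForce clears it.
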(event `self.ReceiveBeginPlay`
  (`self.SetReceivingComponent`)
  (`self.SetForcers`)
  (`self.AddToGame`))

(event `self.ReceiveEndPlay`
  (params (EndPlayReason :type "EEndPlayReason Enum" :default "Destroyed"))
  (`self.RemoveFromGame`))

(fn `AddToGame`)

(fn `AddToTickForce`
  (params (Force :type "Vector Structure"))
  (`/Game/Self/Blueprints/BPML_MacroBag.AddToVector` (`self.TickForce`) Force))

(fn `DrawForce`
  (bind _tickforce (`self.TickForce`))
  (bind _returnvalue (`SceneComponent.K2_GetComponentLocation` (`self.ReceivingComponent`)))
  (bind _returnvalue_2 (`KismetMathLibrary.Loge` (`KismetMathLibrary.VSize` _tickforce)))
  (`KismetSystemLibrary.DrawDebugLine` _returnvalue (+ _returnvalue (* (`KismetMathLibrary.Normal` _tickforce) (* _returnvalue_2 100.0))) (struct :`R` 1.0 :`G` 0.956794 :`B` 0.555928 :`A` 1.0) 0.0 (+ _returnvalue_2 0.0)))

(fn `ReceiveFromAll`
  (params (Forcers :type "Array of /Game/Self/Blueprints/Components/Forcers/BPC_Forcer Object Reference (by ref)"))
  (for _array_element Forcers
    (bind _returnvalue (`/Game/Self/Blueprints/Components/Forcers/BPC_Forcer.ForceFunction` _array_element self))
    (`self.AddToTickForce` _returnvalue)
    (`PrimitiveComponent.AddForce` (`self.ReceivingComponent`) _returnvalue "None" false)))

(fn `RemoveFromGame`)

(fn `ResetTickForce`
  (set `self.TickForce` (0.0 0.0 0.0)))

(fn `SetForcers`)

(fn `SetReceivingComponent`
  (bind _asprimitive_component (cast `PrimitiveComponent` (`Actor.K2_GetRootComponent` (`self.GetOwner`)))
    (:`then`
      (bind _output_get (set `self.ReceivingComponent` _asprimitive_component))
      (`PrimitiveComponent.WakeRigidBody` _output_get "None")
      (`/Game/Self/Blueprints/BPML_MacroBag.PrintStatement` "Waking" (`KismetSystemLibrary.GetDisplayName` _output_get) "" " " false false (struct :`R` 0.76 :`G` 0.100068 :`B` 0.261491 :`A` 1.0) 5.0))
    (:`CastFailed`
      (`KismetSystemLibrary.PrintString` (`KismetStringLibrary.Concat_StrStr` "ERROR: " (`KismetSystemLibrary.GetDisplayName` (`self.GetOwner`)) " ForceRecieverComponent: Root is not of type Primitive Component and cannot simulate physics!")))))