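; Forcer component that computes the Lorentz force, Q(E + v × B), on receivers of type BPC_ReceiverLorentz, returning zero for any other receiver.
; ForceFunction combines the receiving component's physics velocity and charge Q with ElectricField and MagneticField, both evaluated from the receiver-to-owner vector and game time.
; Both field functions return zero here, so the force is zero unless they are overridden.
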(event `self.ReceiveBeginPlay`
  (`parent.ReceiveBeginPlay`))

(event `self.ReceiveTick`
  (params (DeltaSeconds :type "Float (single-precision)"))
  (`parent.ReceiveTick` 0.0))

(fn `ElectricField`
  (params (R :type "Vector Structure") (T :type "Float (double-precision)"))
  (returns (E :type "Vector Structure"))
  (return (0.0 0.0 0.0)))

(fn `ForceFunction`
  (params (Receiver :type "/Game/Self/Blueprints/Components/Receivers/BPC_Receiver Object Reference"))
  (returns (ReturnValue :type "Vector Structure"))
  (bind _returnvalue (`KismetSystemLibrary.GetGameTimeInSeconds`))
  (bind _receivingcomponent (`/Game/Self/Blueprints/Components/Receivers/BPC_Receiver.ReceivingComponent` Receiver))
  (bind _returnvalue_2 (- (`Actor.K2_GetActorLocation` (`self.GetOwner`)) (`SceneComponent.K2_GetComponentLocation` _receivingcomponent)))
  (bind _asbpc_receiver_lorentz (cast `/Game/Self/Blueprints/Components/Receivers/BPC_ReceiverLorentz` Receiver)
    (:`then`
      (bind _returnvalue_3 (`PrimitiveComponent.GetPhysicsLinearVelocity` _receivingcomponent "None"))
      (bind _e (`self.ElectricField` _returnvalue_2 _returnvalue))
      (bind _b (`self.MagneticField` _returnvalue_2 _returnvalue))
      (return (* (+ _e (`KismetMathLibrary.Cross_VectorVector` _returnvalue_3 _b)) (`/Game/Self/Blueprints/Components/Receivers/BPC_ReceiverLorentz.Q` _asbpc_receiver_lorentz))))
    (:`CastFailed`
      (return (0.0 0.0 0.0)))))

(fn `MagneticField`
  (params (R :type "Vector Structure") (T :type "Float (double-precision)"))
  (returns (B :type "Vector Structure"))
  (return (0.0 0.0 0.0)))