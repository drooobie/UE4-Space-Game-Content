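; Radial forcer component that computes a force vector on a receiver along the line toward its owning actor, so positive magnitudes attract.
; ForceFunction measures the distance, optionally clamps it to the inner or outer radius, and returns zero when out of range.
; In range, it normalizes the distance to the band or offsets it by the source radius, with optional inversion.
; RadialFunction supplies the magnitude, returning zero here as an apparent override hook.
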(event EventBeginPlay
  (|CallParentFunction))

(event EventTick
  (params (DeltaSeconds :type Float%20%28single-precision%29))
  (|CallParentFunction 0.0))

(fn RadialFunction
  (params (R :type Float%20%28single-precision%29))
  (return 0.0))

(fn ForceFunction
  (params (Receiver :type BPC%20Receiver%20Object%20Reference))
  (bind _returnvalue (Components|GetOwner))
  (bind _receivingcomponent (Variables|/Game/Self/Blueprints/Components/Receivers/BPC_Receiver.BPC_Receiver_C|GetReceivingComponent Receiver))
  (bind _returnvalue_2 (Transformation|GetWorldLocation _receivingcomponent))
  (bind _returnvalue_3 (Transformation|GetActorLocation _returnvalue))
  (Utilities|FlowControl|Sequence
    (:then_0
      (LocalVariables|SetRUnitVec (Math|Vector|Normalize (- _returnvalue_3 _returnvalue_2)))
      (LocalVariables|SetR (Utilities|Distance(vector) _returnvalue_3 _returnvalue_2)))
    (:then_1
      (if (and (Variables|Default|GetClampToInner) (< (LocalVariables|GetR) (Variables|Default|GetInnerRadius)))
        (LocalVariables|SetR (Variables|Default|GetInnerRadius)))
      (if (and (Variables|Default|GetClampToOuter) (> (LocalVariables|GetR) (Variables|Default|GetOuterRadius)))
        (LocalVariables|SetR (Variables|Default|GetOuterRadius))))
    (:then_2
      (if (Math|Float|InRange(Float) (LocalVariables|GetR) (Variables|Default|GetInnerRadius) (Variables|Default|GetOuterRadius))
        (if (Variables|Default|GetScaleToUnitDisk)
          (LocalVariables|SetR (/ (- (LocalVariables|GetR) (Variables|Default|GetInnerRadius)) (- (Variables|Default|GetOuterRadius) (Variables|Default|GetInnerRadius))))
          (else
            (LocalVariables|SetR (- (LocalVariables|GetR) (Variables|Default|GetSourceRadius)))))
        (if (Variables|Default|GetInvertUnitDisk)
          (LocalVariables|SetR (- 1.0 (LocalVariables|GetR))))
        (else
          (return "0, 0, 0"))))
    (:then_3
      (bind _returnvalue_4 (CallFunction|RadialFunction (LocalVariables|GetR)))
      (return (* (LocalVariables|GetRUnitVec) _returnvalue_4)))))