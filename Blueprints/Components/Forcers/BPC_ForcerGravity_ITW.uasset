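; Gravity forcer component that applies mass-based gravitational force to the game's receiver components.
; On joining the game it registers in the game state's Forcers, takes its gravity scale factor and binds to the pre-physics tick dispatcher, undoing registration and binding on removal.
; Each tick it pushes force to all game-state receivers.
; Its force function multiplies the parent's result by both masses, returning zero for non-static-mesh receivers.
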(event `self.ReceiveBeginPlay`
  (`parent.ReceiveBeginPlay`))

(event `self.ReceiveTick`
  (params (DeltaSeconds :type "Float (single-precision)")))

(event `self.AddToGame`
  (bind _asbp_game_state_itw (cast `/Game/Self/Blueprints/Gameplay/BP_GameState_ITW` (`GameplayStatics.GetGameState`)))
  (`KismetArrayLibrary.Array_Add` (`/Game/Self/Blueprints/Gameplay/BP_GameState_ITW.Forcers` _asbp_game_state_itw) self)
  (set `self.ScaleFactor` (`/Game/Self/Blueprints/Gameplay/BP_GameState_ITW.GravityScaleFactor` _asbp_game_state_itw))
  (add `/Game/Self/Blueprints/Engine/BP_GameTickHandler.Dispatch1` (`/Game/Self/Blueprints/Gameplay/BP_GameState_ITW.TickPrePhysics` _asbp_game_state_itw) (delegate `TickH`)))

(event `TickH`
  (params (TickingGroup :type "ETickingGroup Enum") (Subgroup :type Integer))
  (`self.AddForceToAll` (`/Game/Self/Blueprints/Gameplay/BP_GameState_ITW.Receivers` (stale `self.AddToGame` _asbp_game_state_itw))))

(event `self.RemoveFromGame`
  (bind _asbp_game_state_itw (cast `/Game/Self/Blueprints/Gameplay/BP_GameState_ITW` (`GameplayStatics.GetGameState`)))
  (`KismetArrayLibrary.Array_RemoveItem` (`/Game/Self/Blueprints/Gameplay/BP_GameState_ITW.Forcers` _asbp_game_state_itw) self)
  (remove `/Game/Self/Blueprints/Engine/BP_GameTickHandler.Dispatch1` (`/Game/Self/Blueprints/Gameplay/BP_GameState_ITW.TickPrePhysics` _asbp_game_state_itw) (delegate `TickH`)))

(event `self.SetReceivers`
  (bind _asbp_game_state_itw (cast `/Game/Self/Blueprints/Gameplay/BP_GameState_ITW` (`GameplayStatics.GetGameState`)))
  (set `self.Receivers` (`/Game/Self/Blueprints/Gameplay/BP_GameState_ITW.Receivers` _asbp_game_state_itw)))

(fn `ForceFunction`
  (params (Receiver :type "/Game/Self/Blueprints/Components/Receivers/BPC_Receiver Object Reference"))
  (returns (ReturnValue :type "Vector Structure"))
  (bind _asstatic_mesh_component (cast `StaticMeshComponent` (`/Game/Self/Blueprints/Components/Receivers/BPC_Receiver.ReceivingComponent` Receiver))
    (:`then`
      (bind _returnvalue (`parent.ForceFunction` Receiver))
      (return (* _returnvalue (* (`self.Mass`) (`PrimitiveComponent.GetMass` _asstatic_mesh_component)))))
    (:`CastFailed`
      (return (0.0 0.0 0.0)))))