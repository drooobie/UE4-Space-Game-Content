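; BPC_Forcer is a base component for objects that apply forces to receiver components.
; On BeginPlay it becomes a tick prerequisite of its owner, registers and gathers receivers through empty stub functions, then deregisters on EndPlay.
; ForceFunction returns zero as a placeholder for child classes.
; When active, AddForceToAll evaluates it per receiver, then adds the result to each active receiver's tick force and physics component.
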(event EventBeginPlay
  (Class|Actor|AddTickPrerequisiteComponent (Components|GetOwner) self)
  (CallFunction|AddtoGame)
  (CallFunction|SetReceivers))

(event EventTick
  (params (DeltaSeconds :type Float%20%28single-precision%29)))

(event EventEndPlay
  (params (EndPlayReason :type EEndPlayReason%20Enum :default "Destroyed"))
  (CallFunction|RemovefromGame))

(fn ForceFunction
  (params (Receiver :type BPC%20Receiver%20Object%20Reference))
  (return ""))

(fn SetReceivers)

(fn AddtoGame)

(fn RemovefromGame)

(fn AddForcetoAll
  (params (Receivers :type Array%20of%20BPC%20Receiver%20Object%20References))
  (if (Components|Activation|IsActive)
    (for _array_element Receivers
      (bind _returnvalue (CallFunction|ForceFunction _array_element))
      (if (Components|Activation|IsActive _array_element)
        (Default|AddtoTickForce _array_element _returnvalue)
        (Physics|AddForce (Variables|/Game/Self/Blueprints/Components/Receivers/BPC_Receiver.BPC_Receiver_C|GetReceivingComponent _array_element) _returnvalue "None" false)))))